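; Mutant monster character that wanders the navmesh and shows its name and health on a widget.
; On BeginPlay it starts a self-calling move event that walks to a random reachable point nearby, waits a random few seconds and repeats, continuing only when a move succeeds.
; UpdateUI, also called at BeginPlay, caches the MutantUI from its widget component and fills in the name and health bar.
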(event Custom|怪物移动
  ;[1 1 1] 怪物移动
  (AI|AIMoveTo self (.RandomLocation (Class|NavigationSystemV1|GetRandomPointinNavigableRadius (Transformation|GetActorLocation) 1e+03 0 "/Script/AIModule.NavFilter_AIControllerDefault")) 0 5.0 false
    (:OnSuccess
      (Utilities|FlowControl|Delay (Math|Random|RandomFloatinRange 2.0 5.0))
      (CallFunction|怪物移动))))

(event EventBeginPlay
  ;[1 1 1] 怪物移动
  (CallFunction|怪物移动)
  (CallFunction|UpdateUI))

(fn ConstructionScript)

(fn UpdateUI
  (bind _asmutant_ui (Utilities|Casting|CastToMutantUI (UserInterface|GetUserWidgetObject (Variables|Default|Getwidget))))
  (bind _output_get (Variables|Default|SetMutant%20UI _asmutant_ui))
  (Variables|/Game/Charactor/Monster/Mutant/Blueprint/MutantUI.MutantUI_C|SetMutantName _output_get (Utilities|Text|ToText(String) (Variables|Default|GetName)))
  (Progress|SetPercent (Variables|/Game/Charactor/Monster/Mutant/Blueprint/MutantUI.MutantUI_C|GetHealth _output_get) (Math|Conversions|ToFloat(Integer) (/ (Variables|Default|GetCurrentHealth) (Variables|Default|GetMaxhealth)))))