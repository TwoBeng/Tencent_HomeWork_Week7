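; Weapon_BP is a pickup weapon actor that a player character can take by pressing F.
; Sphere overlap with an ASP_Character stores that character, allows pickup and enables player input; end overlap clears the reference and flag but leaves input enabled.
; F then passes the weapon to the character's 捡取武器 (pick up weapon) function.
; The construction script writes the actor's own class into WeaponInfo, preserving its other fields.
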(event OnComponentEndOverlap(Sphere)
  (params (OverlappedComponent :type Primitive%20Component%20Object%20Reference) (OtherActor :type Actor%20Object%20Reference) (OtherComp :type Primitive%20Component%20Object%20Reference) (OtherBodyIndex :type Integer))
  (Variables|Default|SetASP%20Character%20Ref 0)
  (Variables|Default|SetCan%20Pick%20Up false))

(event OnComponentBeginOverlap(Sphere)
  (params (OverlappedComponent :type Primitive%20Component%20Object%20Reference) (OtherActor :type Actor%20Object%20Reference) (OtherComp :type Primitive%20Component%20Object%20Reference) (OtherBodyIndex :type Integer) (bFromSweep :type Boolean) (SweepResult :type Hit%20Result%20Structure%20%28by%20ref%29))
  (bind _asasp_character (Utilities|Casting|CastToASP_Character OtherActor))
  (Variables|Default|SetASP%20Character%20Ref _asasp_character)
  (Variables|Default|SetCan%20Pick%20Up true)
  (Input|EnableInput (Game|GetPlayerController 0)))

(event EventBeginPlay)

(event Collision|EventActorBeginOverlap
  (params (OtherActor :type Actor%20Object%20Reference)))

(event EventTick
  (params (DeltaSeconds :type Float%20%28single-precision%29)))

(event Input|KeyboardEvents|F
  (params (Key :type Key%20Structure :default "None"))
  (bind _asp_character_ref (Variables|Default|GetASP%20Character%20Ref))
  (:Pressed
    (Utilities|IsValid _asp_character_ref
      (:Is%20Valid
        (if (Variables|Default|GetCan%20Pick%20Up)
          (Default|捡取武器 _asp_character_ref self))))))

(fn ConstructionScript
  (Variables|Default|SetWeaponInfo (Utilities|Struct|MakeWeaponInfo (.weapontype (Variables|Default|GetWeaponInfo)) (Utilities|GetClass self) (.ui (Variables|Default|GetWeaponInfo)) (.name (Variables|Default|GetWeaponInfo)) (.射击速度 (Variables|Default|GetWeaponInfo)) (.开火声音 (Variables|Default|GetWeaponInfo)) (.弹夹装弹量 (Variables|Default|GetWeaponInfo)) (.当前装弹量 (Variables|Default|GetWeaponInfo)) (.武器伤害值 (Variables|Default|GetWeaponInfo)) (.weaponholdsocket (Variables|Default|GetWeaponInfo)) (.weaponequipsocket (Variables|Default|GetWeaponInfo)) (.holdsound (Variables|Default|GetWeaponInfo)) (.equipspund (Variables|Default|GetWeaponInfo)))))